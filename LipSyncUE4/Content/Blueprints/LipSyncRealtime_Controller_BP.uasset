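; Real-time lip sync controller that drives facial morph targets on a Genesis 8 skeletal mesh from JSON received over UDP.
; BeginPlay snapshots the default values of morphs listed in a name-mapping dictionary.
; Each packet first eases all morphs toward those defaults, then applies Phoneme or Expression entries through the dictionary, with debug prints.
; FInterpTo smoothing advances only when packets arrive, as there is no Tick.
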(event `self.ReceiveBeginPlay`
  (`self.SetMorphPlayerDefaultState` (`self.MorphPlayerDefaultState`) (`self.Genesis8Player`))
  (`self.MorphPlayerDefaultStatePrintDebig` (`self.MorphPlayerDefaultState`)))

(event `self.UDP.OnReceivedBytes`
  (params (Bytes :type "Array of Byte (by ref)") (IPAddress :type String))
  (`self.ResetMorphPlayer`)
  (for _array_element (`SIOJLibrary.StringToJsonValueArray` (`CUBlueprintLibrary.Conv_BytesToString` Bytes))
    (bind _returnvalue (`SIOJsonValue.AsObject` _array_element))
    (switch `string` (`SIOJsonObject.GetStringField` _returnvalue "Type")
      (:`Phoneme`
        (bind _returnvalue_2 (`SIOJsonObject.GetObjectField` _returnvalue "Value"))
        (bind _returnvalue_3 (`SIOJsonObject.GetStringField` _returnvalue_2 "Name"))
        (bind _returnvalue_4 (`SIOJsonObject.GetNumberField` _returnvalue_2 "Value"))
        (`KismetSystemLibrary.PrintString` (`KismetStringLibrary.Concat_StrStr` _returnvalue_3 "|" (`KismetStringLibrary.Conv_DoubleToString` _returnvalue_4)))
        (`self.SetPlayerMorph` (`self.Genesis8Player`) (`self.MorphPlayerDictionary`) (`self.SmoothSpeed`) _returnvalue_3 _returnvalue_4))
      (:`Expression`
        (bind _returnvalue_5 (`SIOJsonObject.GetArrayField` _returnvalue "Value"))
        (for _array_element_2 _returnvalue_5
          (bind _returnvalue_6 (`SIOJsonValue.AsObject` _array_element_2))
          (bind _returnvalue_7 (`SIOJsonObject.GetStringField` _returnvalue_6 "Name"))
          (bind _returnvalue_8 (`SIOJsonObject.GetNumberField` _returnvalue_6 "Value"))
          (`KismetSystemLibrary.PrintString` (`KismetStringLibrary.Concat_StrStr` _returnvalue_7 "|" (`KismetStringLibrary.Conv_DoubleToString` _returnvalue_8)))
          (`self.SetPlayerMorph` (`self.Genesis8Player`) (`self.MorphPlayerDictionary`) (`self.SmoothSpeed`) _returnvalue_7 _returnvalue_8))))))

(event `ResetMorphPlayer`
  (`self.SetPlayerMorphArray` (`self.MorphPlayerDefaultState`) (`self.Genesis8Player`) (`self.SmoothSpeed`)))

(fn `GetPlayerMorphValue`
  (params (MorphPlayerName :type String) (SkeletalMeshPlayer :type "SkeletalMeshActor Object Reference"))
  (returns (Value :type "Float (double-precision)"))
  (return (`SkeletalMeshComponent.GetMorphTarget` (`SkeletalMeshActor.SkeletalMeshComponent` SkeletalMeshPlayer) (`KismetStringLibrary.Conv_StringToName` MorphPlayerName))))

(fn `MorphPlayerDefaultStatePrintDebig`
  (params (MorphPlayerDefaultState :type "Map of String to Float (double-precision)"))
  (bind _keys (`BlueprintMapLibrary.Map_Keys` MorphPlayerDefaultState))
  (for _array_element _keys
    (`KismetSystemLibrary.PrintString` (`KismetStringLibrary.Concat_StrStr` "Morph name: " _array_element " Value: " (`KismetStringLibrary.Conv_DoubleToString` (`BlueprintMapLibrary.Map_Find` MorphPlayerDefaultState _array_element))))))

(fn `SetMorphPlayerDefaultState`
  (params (MorphPlayerDefaultState :type "Map of String to Float (double-precision) (by ref)") (SkeletalMeshPlayer :type "SkeletalMeshActor Object Reference (by ref)"))
  (returns (Result :type "Map of String to Float (double-precision)"))
  (`BlueprintMapLibrary.Map_Clear` MorphPlayerDefaultState)
  (bind _values (`BlueprintMapLibrary.Map_Values` (`self.MorphPlayerDictionary`)))
  (for _array_element _values
    (bind _value (`self.GetPlayerMorphValue` _array_element SkeletalMeshPlayer))
    (`BlueprintMapLibrary.Map_Add` MorphPlayerDefaultState _array_element _value))
  (return MorphPlayerDefaultState))

(fn `SetPlayerMorph`
  (params (SkeletalMeshPlayer :type "SkeletalMeshActor Object Reference (by ref)") (MorphPlayerDictionary :type "Map of String to String") (SmoothSpeed :type "Float (double-precision)" :default 10.0) (MorphName :type String) (MorphValue :type "Float (double-precision)"))
  (bind (_value _returnvalue) (`BlueprintMapLibrary.Map_Find` MorphPlayerDictionary MorphName))
  (if _returnvalue
    (bind _value_2 (`self.GetPlayerMorphValue` _value SkeletalMeshPlayer))
    (`SkeletalMeshComponent.SetMorphTarget` (`SkeletalMeshActor.SkeletalMeshComponent` SkeletalMeshPlayer) (`KismetStringLibrary.Conv_StringToName` _value) (`KismetMathLibrary.FInterpTo` _value_2 MorphValue (`GameplayStatics.GetWorldDeltaSeconds`) SmoothSpeed) true)))

(fn `SetPlayerMorphArray`
  (params (MorphPlayerTrackTickState :type "Map of String to Float (double-precision)") (SkeletalMeshPlayer :type "SkeletalMeshActor Object Reference (by ref)") (SmoothSpeed :type "Float (double-precision)" :default 10.0))
  (bind _keys (`BlueprintMapLibrary.Map_Keys` MorphPlayerTrackTickState))
  (for _array_element _keys
    (bind _value (`self.GetPlayerMorphValue` _array_element SkeletalMeshPlayer))
    (`SkeletalMeshComponent.SetMorphTarget` (`SkeletalMeshActor.SkeletalMeshComponent` SkeletalMeshPlayer) (`KismetStringLibrary.Conv_StringToName` _array_element) (`KismetMathLibrary.FInterpTo` _value (`BlueprintMapLibrary.Map_Find` MorphPlayerTrackTickState _array_element) (`GameplayStatics.GetWorldDeltaSeconds`) SmoothSpeed) true)))

(fn `UserConstructionScript`)