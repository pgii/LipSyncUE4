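; Lip-sync controller that animates a Genesis 8 character's facial morph targets and shows timed subtitles from a data table track.
; On BeginPlay it loads phoneme, expression and subtitle tracks, caches default morph values, and creates the subtitle widget.
; Audio playback percent, or a delay loop without audio, advances elapsed time, which selects active entries and eases mapped morphs toward their values.
; When audio ends, it steps morphs toward defaults and clears the subtitle.
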(event `self.ReceiveBeginPlay`
  (`self.InitLipSync`)
  (`self.InitSubtitleWidget`)
  (`self.SetMorphPlayerDefaultState` (`self.MorphPlayerDefaultState`) (`self.Genesis8Player`))
  (`self.MorphPlayerDefaultStatePrintDebig` (`self.MorphPlayerDefaultState`))
  (`/Engine/EditorBlueprintResources/StandardMacros.IsValid` (`self.AudioTrack`)
    (:`Is Valid`
      (`self.PlayAudioTrack`))
    (:`Is Not Valid`
      (`self.PtayTrackWithoutAudio`))))

(event `InitLipSync`
  (`self.FillLipSyncPartStructFromDataTable` (`self.LipSyncPartStruct`) (`self.LipSyncTrackDataTable`))
  (`self.LipSyncPartPrintDebig` (`self.LipSyncPartStruct`)))

(event `InitSubtitleWidget`
  (bind _foundwidgets (`WidgetBlueprintLibrary.GetAllWidgetsOfClass` "/Game/Blueprints/GUI_LipSyncSubtitle_BP.GUI_LipSyncSubtitle_BP_C"))
  (`KismetArrayLibrary.Array_Clear` _foundwidgets)
  (bind _returnvalue (`|CreateWidget` "/Game/Blueprints/GUI_LipSyncSubtitle_BP.GUI_LipSyncSubtitle_BP_C"))
  (bind _output_get (set `self.SubtitleWidget` _returnvalue))
  (`UserWidget.AddToViewport` _output_get 0)
  (`self.ClearWidgetSubtitle`))

(event `StopTrack`
  (`self.SetPlayerMorphArray` (`self.MorphPlayerDefaultState`) (`self.Genesis8Player`))
  (`self.ClearWidgetSubtitle`))

(event `PlayAudioTrack`
  (`/Engine/EditorBlueprintResources/StandardMacros.IsValid` (`self.AudioTrack`)
    (:`Is Valid`
      (bind _returnvalue (`GameplayStatics.SpawnSound2D` (`self.AudioTrack`) 1.0 1.0 0.0 null))
      (bind _output_get (set `self.AudioComponent` _returnvalue))
      (add `AudioComponent.OnAudioPlaybackPercent` _output_get (delegate `AudioPlaybackPercent_Tick`))
      (`AudioComponent.Play` _output_get 0.0))))

(event `AudioPlaybackPercent_Tick`
  (params (PlayingSoundWave :type "SoundWave Object Reference") (PlaybackPercent :type "Float (double-precision)"))
  (if (< PlaybackPercent 1.0)
    (set `self.ElapsedTime` (* (`SoundBase.Duration` PlayingSoundWave) PlaybackPercent))
    (`self.SetMorphTrackTick`)
    (else
      (`self.StopTrack`))))

(event `PtayTrackWithoutAudio`
  (bind _returnvalue (`GameplayStatics.GetWorldDeltaSeconds`))
  (bind _lipsyncpartstruct_audiotrack (break `/Game/Blueprints/LipSyncPartStruct` (`self.LipSyncPartStruct`)))
  (bind (_output_name _output_start _output_end) (break `/Game/Blueprints/LipSyncTrackStruct` (`|GetArrayItem` _lipsyncpartstruct_audiotrack)))
  (bind _output_get (set `self.ElapsedTime` (+ (`self.ElapsedTime`) _returnvalue) :!label _label))
  (if (<= _output_get _output_end)
    (`KismetSystemLibrary.Delay` _returnvalue)
    (`self.SetMorphTrackTick`)
    (`KismetSystemLibrary.PrintString` (`KismetStringLibrary.Conv_DoubleToString` (`self.ElapsedTime`)) true true (struct :`R` 1.0 :`G` 0.711512 :`B` 0.127732 :`A` 1.0))
    (goto _label)))

(event `SetMorphTrackTick`
  (bind _lipsynctrackstruct (`self.GetLipSyncTrackArrayFromTime` (`self.LipSyncPartStruct`) (`self.ElapsedTime`)))
  (`self.LipSyncTrackArrayFromTimePrintDebig` _lipsynctrackstruct)
  (`self.Get Morph Player Track Tick State` _lipsynctrackstruct (`self.ElapsedTime`) (`self.MorphPlayerTrackTickState`) (`self.MorphPlayerDictionary`))
  (`self.MorphPlayerTrackTickStatePrintDebig` (`self.MorphPlayerTrackTickState`))
  (`self.SetPlayerMorphArray` (`self.MorphPlayerTrackTickState`) (`self.Genesis8Player`) (`self.SmoothSpeed`))
  (`self.SetWidgetSubtitle`))

(event `SetWidgetSubtitle`
  (bind _subtitle (`self.GetLipSyncSubtitleFromTime` (`self.LipSyncPartStruct`) (`self.ElapsedTime`)))
  (`TextBlock.SetText` (`/Game/Blueprints/GUI_LipSyncSubtitle_BP.tbSubtitle` (`self.SubtitleWidget`)) (`KismetTextLibrary.Conv_StringToText` _subtitle)))

(event `ClearWidgetSubtitle`
  (`TextBlock.SetText` (`/Game/Blueprints/GUI_LipSyncSubtitle_BP.tbSubtitle` (`self.SubtitleWidget`)) ""))

(fn `FillLipSyncPartStructFromDataTable`
  (params (LipSyncPartStruct :type "/Game/Blueprints/LipSyncPartStruct Structure (by ref)") (LipSyncTrackDataTable :type "DataTable Object Reference"))
  (returns (Result :type "/Game/Blueprints/LipSyncPartStruct Structure"))
  (bind (_audiotrack _phoneme) (break `/Game/Blueprints/LipSyncPartStruct` LipSyncPartStruct))
  (bind _audiotrack_2 (break `/Game/Blueprints/LipSyncPartStruct` LipSyncPartStruct))
  (bind (_audiotrack_3 _phoneme_2 _expression) (break `/Game/Blueprints/LipSyncPartStruct` LipSyncPartStruct))
  (bind (_audiotrack_4 _phoneme_3 _expression_2 _subtitle) (break `/Game/Blueprints/LipSyncPartStruct` LipSyncPartStruct))
  (bind _outrownames (`DataTableFunctionLibrary.GetDataTableRowNames` LipSyncTrackDataTable))
  (for _array_element _outrownames
    (switch `name` _array_element
      (:`AudioTrack`
        (bind _returnvalue (`|GetDataTableRow` LipSyncTrackDataTable _array_element)
          (:`then`
            (`KismetArrayLibrary.Array_Clear` _audiotrack_2)
            (for _array_element_2 (`.Value_6_DEF7FB10487B98D59928CD89559C3803` (break `/Game/Blueprints/LipSyncImportStruct` _returnvalue))
              (`KismetArrayLibrary.Array_Add` _audiotrack_2 _array_element_2)))))
      (:`Phoneme`
        (bind _returnvalue_2 (`|GetDataTableRow` LipSyncTrackDataTable _array_element)
          (:`then`
            (`KismetArrayLibrary.Array_Clear` _phoneme)
            (for _array_element_3 (`.Value_6_DEF7FB10487B98D59928CD89559C3803` (break `/Game/Blueprints/LipSyncImportStruct` _returnvalue_2))
              (`KismetArrayLibrary.Array_Add` _phoneme _array_element_3)))))
      (:`Expression`
        (bind _returnvalue_3 (`|GetDataTableRow` LipSyncTrackDataTable _array_element)
          (:`then`
            (`KismetArrayLibrary.Array_Clear` _expression)
            (for _array_element_4 (`.Value_6_DEF7FB10487B98D59928CD89559C3803` (break `/Game/Blueprints/LipSyncImportStruct` _returnvalue_3))
              (`KismetArrayLibrary.Array_Add` _expression _array_element_4)))))
      (:`Subtitle`
        (bind _returnvalue_4 (`|GetDataTableRow` LipSyncTrackDataTable _array_element)
          (:`then`
            (`KismetArrayLibrary.Array_Clear` _subtitle)
            (for _array_element_5 (`.Value_6_DEF7FB10487B98D59928CD89559C3803` (break `/Game/Blueprints/LipSyncImportStruct` _returnvalue_4))
              (`KismetArrayLibrary.Array_Add` _subtitle _array_element_5)))))))
  (return LipSyncPartStruct))

(fn `Get Morph Player Track Tick State`
  (params (LipSyncTrackStructArray :type "Array of /Game/Blueprints/LipSyncTrackStruct Structure") (ElapsedTime :type "Float (double-precision)") (MorphPlayerTrackTickState :type "Map of String to Float (double-precision) (by ref)") (MorphPlayerDictionary :type "Map of String to String"))
  (returns (Result :type "Map of String to Float (double-precision)"))
  (locals (LocalLipSyncTrackStruct :type "Array of /Game/Blueprints/LipSyncTrackStruct Structure") (LocalElapsedTime :type "Float (double-precision)"))
  (set `local.LocalElapsedTime` ElapsedTime)
  (bind _keys (`BlueprintMapLibrary.Map_Keys` MorphPlayerDictionary))
  (for _array_element _keys
    (bind _value (`BlueprintMapLibrary.Map_Find` MorphPlayerDictionary _array_element))
    (`BlueprintMapLibrary.Map_Add` MorphPlayerTrackTickState _value)
    (for _array_element_2 LipSyncTrackStructArray
      (bind (_name _start _end _value_2) (break `/Game/Blueprints/LipSyncTrackStruct` _array_element_2))
      (if (`KismetStringLibrary.EqualEqual_StrStr` _array_element (`KismetTextLibrary.Conv_TextToString` _name))
        (`BlueprintMapLibrary.Map_Add` MorphPlayerTrackTickState _value _value_2))))
  (return MorphPlayerTrackTickState))

(fn `GetLipSyncSubtitleFromTime`
  (params (LipSyncPartStruct :type "/Game/Blueprints/LipSyncPartStruct Structure") (ElapsedTime :type "Float (double-precision)"))
  (returns (Subtitle :type String))
  (locals (LocalElapsedTime :type "Float (double-precision)"))
  (set `local.LocalElapsedTime` ElapsedTime)
  (for _array_element (`.Subtitle_30_4FCB621643F2F63A35972C8CFABC5B25` (break `/Game/Blueprints/LipSyncPartStruct` LipSyncPartStruct))
    (bind (_name _start _end) (break `/Game/Blueprints/LipSyncTrackStruct` _array_element))
    (if (and (>= (`local.LocalElapsedTime`) _start) (<= (`local.LocalElapsedTime`) _end))
      (return (`KismetTextLibrary.Conv_TextToString` _name))))
  (return ""))

(fn `GetLipSyncTrackArrayFromTime`
  (params (LipSyncPartStruct :type "/Game/Blueprints/LipSyncPartStruct Structure") (ElapsedTime :type "Float (double-precision)"))
  (returns (LipSyncTrackStruct :type "Array of /Game/Blueprints/LipSyncTrackStruct Structure"))
  (locals (LocalLipSyncTrackStruct :type "Array of /Game/Blueprints/LipSyncTrackStruct Structure") (LocalElapsedTime :type "Float (double-precision)"))
  (bind (_audiotrack _phoneme _expression) (break `/Game/Blueprints/LipSyncPartStruct` LipSyncPartStruct))
  (set `local.LocalElapsedTime` ElapsedTime)
  (for _array_element _phoneme
    (bind (_name _start _end) (break `/Game/Blueprints/LipSyncTrackStruct` _array_element))
    (if (and (>= (`local.LocalElapsedTime`) _start) (<= (`local.LocalElapsedTime`) _end))
      (`KismetArrayLibrary.Array_Add` (`local.LocalLipSyncTrackStruct`) _array_element)))
  (for _array_element_2 _expression
    (bind (_name_2 _start_2 _end_2) (break `/Game/Blueprints/LipSyncTrackStruct` _array_element_2))
    (if (and (>= (`local.LocalElapsedTime`) _start_2) (<= (`local.LocalElapsedTime`) _end_2))
      (`KismetArrayLibrary.Array_Add` (`local.LocalLipSyncTrackStruct`) _array_element_2)))
  (return (`local.LocalLipSyncTrackStruct`)))

(fn `GetPlayerMorphValue`
  (params (MorphPlayerName :type String) (SkeletalMeshPlayer :type "SkeletalMeshActor Object Reference"))
  (returns (Value :type "Float (double-precision)"))
  (return (`SkeletalMeshComponent.GetMorphTarget` (`SkeletalMeshActor.SkeletalMeshComponent` SkeletalMeshPlayer) (`KismetStringLibrary.Conv_StringToName` MorphPlayerName))))

(fn `LipSyncPartPrintDebig`
  (params (LipSyncPartStruct :type "/Game/Blueprints/LipSyncPartStruct Structure"))
  (bind (_audiotrack _phoneme _expression _subtitle) (break `/Game/Blueprints/LipSyncPartStruct` LipSyncPartStruct))
  (for _array_element _phoneme
    (`self.LipSyncTrackPrintDebig` _array_element))
  (for _array_element_2 _expression
    (`self.LipSyncTrackPrintDebig` _array_element_2))
  (for _array_element_3 _subtitle
    (`self.LipSyncTrackPrintDebig` _array_element_3))
  (return))

(fn `LipSyncTrackArrayFromTimePrintDebig`
  (params (LipSyncTrackStructArray :type "Array of /Game/Blueprints/LipSyncTrackStruct Structure"))
  (for _array_element LipSyncTrackStructArray
    (bind (_name _start _end _value) (break `/Game/Blueprints/LipSyncTrackStruct` _array_element))
    (`KismetSystemLibrary.PrintString` (`KismetStringLibrary.Concat_StrStr` "Name: " (`KismetTextLibrary.Conv_TextToString` _name) " Start: " (`KismetStringLibrary.Conv_DoubleToString` _start) " End: " (`KismetStringLibrary.Conv_DoubleToString` _end) " Value: " (`KismetStringLibrary.Conv_DoubleToString` _value)) true true (struct :`R` 1.0 :`G` 0.115454 :`A` 1.0))))

(fn `LipSyncTrackPrintDebig`
  (params (LipSyncTrackStruct :type "/Game/Blueprints/LipSyncTrackStruct Structure"))
  (bind (_name _start _end _value) (break `/Game/Blueprints/LipSyncTrackStruct` LipSyncTrackStruct))
  (`KismetSystemLibrary.PrintString` (`KismetStringLibrary.Concat_StrStr` "Name: " (`KismetTextLibrary.Conv_TextToString` _name) " Start: " (`KismetStringLibrary.Conv_DoubleToString` _start) " End: " (`KismetStringLibrary.Conv_DoubleToString` _end) " Value: " (`KismetStringLibrary.Conv_DoubleToString` _value))))

(fn `MorphPlayerDefaultStatePrintDebig`
  (params (MorphPlayerDefaultState :type "Map of String to Float (double-precision)"))
  (bind _keys (`BlueprintMapLibrary.Map_Keys` MorphPlayerDefaultState))
  (for _array_element _keys
    (`KismetSystemLibrary.PrintString` (`KismetStringLibrary.Concat_StrStr` "Morph name: " _array_element " Value: " (`KismetStringLibrary.Conv_DoubleToString` (`BlueprintMapLibrary.Map_Find` MorphPlayerDefaultState _array_element))))))

(fn `MorphPlayerTrackTickStatePrintDebig`
  (params (LipSyncTrackStructArray :type "Map of String to Float (double-precision)"))
  (bind _keys (`BlueprintMapLibrary.Map_Keys` LipSyncTrackStructArray))
  (for _array_element _keys
    (`KismetSystemLibrary.PrintString` (`KismetStringLibrary.Concat_StrStr` "Name: " _array_element " Value: " (`KismetStringLibrary.Conv_DoubleToString` (`BlueprintMapLibrary.Map_Find` LipSyncTrackStructArray _array_element))) true true (struct :`R` 1.0 :`G` 1.0 :`B` 1.0 :`A` 1.0))))

(fn `SetMorphPlayerDefaultState`
  (params (MorphPlayerDefaultState :type "Map of String to Float (double-precision) (by ref)") (SkeletalMeshPlayer :type "SkeletalMeshActor Object Reference (by ref)"))
  (returns (Result :type "Map of String to Float (double-precision)"))
  (`BlueprintMapLibrary.Map_Clear` MorphPlayerDefaultState)
  (bind _values (`BlueprintMapLibrary.Map_Values` (`self.MorphPlayerDictionary`)))
  (for _array_element _values
    (bind _value (`self.GetPlayerMorphValue` _array_element SkeletalMeshPlayer))
    (`BlueprintMapLibrary.Map_Add` MorphPlayerDefaultState _array_element _value))
  (return MorphPlayerDefaultState))

(fn `SetPlayerMorphArray`
  (params (MorphPlayerTrackTickState :type "Map of String to Float (double-precision)") (SkeletalMeshPlayer :type "SkeletalMeshActor Object Reference (by ref)") (SmoothSpeed :type "Float (double-precision)" :default 10.0))
  (bind _keys (`BlueprintMapLibrary.Map_Keys` MorphPlayerTrackTickState))
  (for _array_element _keys
    (bind _value (`self.GetPlayerMorphValue` _array_element SkeletalMeshPlayer))
    (`SkeletalMeshComponent.SetMorphTarget` (`SkeletalMeshActor.SkeletalMeshComponent` SkeletalMeshPlayer) (`KismetStringLibrary.Conv_StringToName` _array_element) (`KismetMathLibrary.FInterpTo` _value (`BlueprintMapLibrary.Map_Find` MorphPlayerTrackTickState _array_element) (`GameplayStatics.GetWorldDeltaSeconds`) SmoothSpeed) true)))

(fn `UserConstructionScript`)